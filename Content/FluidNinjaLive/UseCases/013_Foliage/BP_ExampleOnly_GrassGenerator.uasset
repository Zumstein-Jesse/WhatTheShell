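; Example grass generator actor that scatters instanced static mesh clumps at BeginPlay and links their material to a FluidNinja fluid simulation.
; Clumps use an ordered, jittered grid or a randomized spread, with optional centering and random yaw and scale.
; A dynamic grass material receives trace mesh position and size from a parameter collection every tick through a gate, plus the velocity/density render target once.
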(event EventBeginPlay
  (bind _returnvalue (Utilities|Name|MakeLiteralName "TraceMeshSize"))
  (bind _returnvalue_2 (Utilities|Name|MakeLiteralName "TraceMeshPos"))
  (bind _averagedistancebetweenclumps (Variables|GrassGeneratorParams|GetAverageDistanceBetweenClumps))
  (bind _averagedistancebetweenclumps_2 (Variables|GrassGeneratorParams|GetAverageDistanceBetweenClumps))
  (bind _materialparamcollection (Variables|XFluidsimDataFromExternalSystem|GetMaterialParamCollection))
  (bind _grassmaterial (Variables|XFluidsimDataFromExternalSystem|GetGrassMaterial))
  (bind _rendertarget (Variables|XFluidsimDataFromExternalSystem|GetRenderTarget))
  (bind _numberofgrassclumps (Variables|GrassGeneratorParams|GetNumberOfGrassClumps))
  (bind _returnvalue_3 (Math|Conversions|ToFloat(Integer) _numberofgrassclumps))
  (bind _returnvalue_4 (Math|Float|Sqrt _returnvalue_3))
  (bind _returnvalue_5 (Math|Float|Round _returnvalue_4))
  (bind _returnvalue_6 (* _averagedistancebetweenclumps _returnvalue_4))
  (bind _returnvalue_7 (* _returnvalue_6 -0.5))
  (Utilities|FlowControl|Sequence
    (:then_0
      (if (not (Variables|GrassGeneratorParams|GetDisableGrassGenerator))
        (for _index (range 0 (Variables|GrassGeneratorParams|GetNumberOfGrassClumps))
          (Utilities|Array|Add (Variables|GrassGeneratorParams|GetInstance%20Transforms) (Math|Transform|MakeTransform (+ (* (Math|Vector|MakeVector _returnvalue_7 _returnvalue_7 0.0) (Math|Conversions|ToFloat(Boolean) (Variables|GrassGeneratorParams|GetCenteredPlacement))) (Math|Vector|SelectVector (+ (* (Math|Random|RandomUnitVector) (Variables|GrassGeneratorParams|GetRandomizeGrassClumpPosition)) (Math|Vector|MakeVector (* (Math|Conversions|ToFloat(Integer) (Math|Integer|%(Integer) _index _returnvalue_5)) _averagedistancebetweenclumps_2) (* _averagedistancebetweenclumps_2 (Math|Conversions|ToFloat(Integer) (/ _index _returnvalue_5))) 0.0)) (* (+ (Math|Random|RandomUnitVector) 0.5) (Math|Vector|MakeVector (* (Math|Float|Power (Math|Conversions|ToFloat(Integer) _index) 0.4) (Variables|GrassGeneratorParams|GetAverageDistanceBetweenClumps)) (* (Math|Float|Power (Math|Conversions|ToFloat(Integer) _index) 0.4) (Variables|GrassGeneratorParams|GetAverageDistanceBetweenClumps)) 0.0)) (Variables|GrassGeneratorParams|GetOrderedPlacementMode))) (Math|Rotator|MakeRotator 0.0 0.0 (* (Math|Float|MultiplybyPi (Math|Random|RandomFloat)) (* (Variables|GrassGeneratorParams|GetRandomizeGrassClumpRotation) 1e+02))) (Math|Conversions|ToVector(Float) (+ (* (Math|Random|RandomFloat) (Variables|GrassGeneratorParams|GetRandomizeGrassClumpScale)) (Variables|GrassGeneratorParams|GetBaseScale))))))
        (Components|InstancedStaticMesh|AddInstances (Variables|Default|GetInstancedStaticMesh) (Variables|GrassGeneratorParams|GetInstance%20Transforms) false)))
    (:then_1
      (Utilities|IsValid _grassmaterial
        (:Is%20Valid
          (bind _returnvalue_8 (Rendering|Material|CreateDynamicMaterialInstance _grassmaterial "None" "None" :!class /Script/Engine.KismetMaterialLibrary))
          (Variables|XFluidsimDataFromExternalSystem|SetGrassMaterialDyamicInstance _returnvalue_8)
          (Rendering|Material|SetMaterial (Variables|Default|GetInstancedStaticMesh) 0 (Variables|XFluidsimDataFromExternalSystem|GetGrassMaterialDyamicInstance))
          ;[0.04985 1 0.4002] Set TraceMesh Position and Scale plus fluidsim VElocity and Density Buffers to Grass Material
          (Utilities|IsValid _materialparamcollection
            (:Is%20Valid
              (Utilities|FlowControl|Gate true) ; enters at Open
            )))))))

(event EventTick
  (params (DeltaSeconds :type Float%20%28single-precision%29))
  (bind _returnvalue (Utilities|Name|MakeLiteralName "TraceMeshSize"))
  (bind _returnvalue_2 (Utilities|Name|MakeLiteralName "TraceMeshPos"))
  (bind _materialparamcollection (Variables|XFluidsimDataFromExternalSystem|GetMaterialParamCollection))
  (bind _rendertarget (Variables|XFluidsimDataFromExternalSystem|GetRenderTarget))
  (bind _grassmaterialdyamicinstance (Variables|XFluidsimDataFromExternalSystem|GetGrassMaterialDyamicInstance))
  ;[0.04985 1 0.4002] Set TraceMesh Position and Scale plus fluidsim VElocity and Density Buffers to Grass Material
  (Utilities|FlowControl|Gate true
    (:Exit
      (bind _returnvalue_3 (Rendering|Material|GetVectorParameterValue _materialparamcollection _returnvalue :!class /Script/Engine.KismetMaterialLibrary))
      (Rendering|Material|SetVectorParameterValue _grassmaterialdyamicinstance _returnvalue _returnvalue_3 :!class /Script/Engine.MaterialInstanceDynamic)
      (bind _returnvalue_4 (Rendering|Material|GetVectorParameterValue _materialparamcollection _returnvalue_2 :!class /Script/Engine.KismetMaterialLibrary))
      (Rendering|Material|SetVectorParameterValue _grassmaterialdyamicinstance _returnvalue_2 _returnvalue_4 :!class /Script/Engine.MaterialInstanceDynamic)
      (Utilities|FlowControl|DoOnce false
        (:Completed
          (Utilities|IsValid _rendertarget
            (:Is%20Valid
              (Rendering|Material|SetTextureParameterValue (Variables|XFluidsimDataFromExternalSystem|GetGrassMaterialDyamicInstance) "VelocityDensityBuffer" _rendertarget))))))))

(fn ConstructionScript)