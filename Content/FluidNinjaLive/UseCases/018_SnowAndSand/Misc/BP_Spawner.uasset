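; Spawner actor for the FluidNinjaLive snow and sand use case that keeps dropping heavy physics spheres into the scene.
; BeginPlay loops on a delay, spawning BP_Sphere at a random X offset with physics, overlap events and a mass override, and appends it to CubeArray.
; Tick uses a longer Delay to periodically destroy the oldest entry, so removal runs slower than spawning and spheres accumulate.
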(event EventBeginPlay
  (bind _self self)
  (bind _returnvalue (Transformation|GetActorTransform _self))
  (bind (_location _rotation _scale) (Math|Transform|BreakTransform _returnvalue))
  (bind (_x _y _z) (Math|Vector|BreakVector _location))
  (bind _returnvalue_2 (Game|SpawnActorfromClass "/Game/FluidNinjaLive/UseCases/018_SnowAndSand/Misc/BP_Sphere.BP_Sphere_C" (Math|Transform|MakeTransform (Math|Vector|MakeVector (+ (Math|Random|RandomFloatinRange -2.5e+02 2.5e+02) _x) _y _z) _rotation _scale) "AlwaysSpawn" 0 0 :!label _label))
  (Rendering|Material|SetMaterial (Variables|/Game/FluidNinjaLive/UseCases/018_SnowAndSand/Misc/BP_Sphere.BP_Sphere_C|GetStaticMesh _returnvalue_2) 0 "/Engine/BasicShapes/BasicShapeMaterial.BasicShapeMaterial")
  (Physics|SetSimulatePhysics (Variables|/Game/FluidNinjaLive/UseCases/018_SnowAndSand/Misc/BP_Sphere.BP_Sphere_C|GetStaticMesh _returnvalue_2) true)
  (Variables|/Script/Engine.PrimitiveComponent|SetbGenerateOverlapEvents (Variables|/Game/FluidNinjaLive/UseCases/018_SnowAndSand/Misc/BP_Sphere.BP_Sphere_C|GetStaticMesh _returnvalue_2) true)
  (Class|PrimitiveComponent|SetMassOverrideinKg (Variables|/Game/FluidNinjaLive/UseCases/018_SnowAndSand/Misc/BP_Sphere.BP_Sphere_C|GetStaticMesh _returnvalue_2) "None" 2e+02 true)
  (Utilities|Array|Add (Variables|Default|GetCubeArray) _returnvalue_2)
  (Utilities|FlowControl|Delay 3.0)
  (goto _label))

(event EventTick
  (params (DeltaSeconds :type Float%20%28single-precision%29))
  (bind _cubearray (Variables|Default|GetCubeArray))
  (bind _output (Utilities|Array|Get(acopy) _cubearray))
  (Utilities|FlowControl|Delay 6.0)
  (Actor|DestroyActor _output)
  (Utilities|Array|RemoveItem _cubearray _output))

(fn ConstructionScript)